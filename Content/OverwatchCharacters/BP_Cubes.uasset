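; BP_Cubes is a cube actor that reacts to snowball and fireball hits.
; A BP_SnowBall hit swaps its material, sets a freeze flag, plays a sound, then after a short delay makes the mesh Static.
; After a few seconds the mesh returns to Movable, takes the fireball material and clears the flag.
; A BP_FireBall hit destroys the cube only while the flag is set.
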(event Custom|FreezeBig
  (Transformation|SetMobility (Variables|Debug|GetStaticMeshComponent) "Static")
  (Utilities|FlowControl|Delay 3.0)
  (Transformation|SetMobility (Variables|Debug|GetStaticMeshComponent) "Movable")
  (Rendering|Material|SetMaterial (Variables|Debug|GetStaticMeshComponent) 0 "/Game/FPWeapon/Materials/FireBallMat.FireBallMat")
  (Variables|Default|SetFreezeBig? false))

(event EventBeginPlay)

(event Collision|EventActorBeginOverlap
  (params (OtherActor :type Actor%20Object%20Reference)))

(event EventTick
  (params (DeltaSeconds :type Float%20%28single-precision%29)))

(event Collision|EventHit
  (params (MyComp :type Primitive%20Component%20Object%20Reference) (Other :type Actor%20Object%20Reference) (OtherComp :type Primitive%20Component%20Object%20Reference) (bSelfMoved :type Boolean) (HitLocation :type Vector :default "0, 0, 0") (HitNormal :type Vector :default "0, 0, 0") (NormalImpulse :type Vector :default "0, 0, 0") (Hit :type Hit%20Result%20Structure%20%28by%20ref%29))
  (Utilities|Casting|CastToBP_SnowBall Other
    (:then
      (Rendering|Material|SetMaterial (Variables|Debug|GetStaticMeshComponent) 0 "/Game/FPWeapon/Materials/SnowBallMat.SnowBallMat")
      (Variables|Default|SetFreezeBig? true)
      (Audio|SpawnSound2D "/Game/Sound/Freeze_-_Sound_Effect_HD.Freeze_-_Sound_Effect_HD" 1.0 1.0 0.0 0)
      (Utilities|FlowControl|Delay 0.5)
      (CallFunction|FreezeBig))
    (:CastFailed
      (Utilities|Casting|CastToBP_FireBall Other)
      (if (Variables|Default|GetFreezeBig?)
        (Actor|DestroyActor)))))

(fn ConstructionScript)