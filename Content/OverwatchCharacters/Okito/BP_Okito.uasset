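; BP_Okito is a playable hero Blueprint with elemental projectile abilities and an upward launch.
; On initialization it adds the Okito input mapping context and shows a tutorial widget briefly; BeginPlay adds a weapon component.
; Freeze and Fire spawn snowball or fireball actors propelled along the camera's forward vector, with sound.
; Ride launches the character upward through a DoOnce whose reset is disconnected, as are older ride-spawn and cube-pushing trace nodes.
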(event Input|EnhancedActionEvents|EnhancedInputActionRide
  (params (ActionValue :type Boolean) (ElapsedSeconds :type Float%20%28double-precision%29) (TriggeredSeconds :type Float%20%28double-precision%29) (InputAction :type Input%20Action%20Object%20Reference :default "/Game/OverwatchCharacters/Okito/Inputs/Ride.Ride"))
  (:Triggered
    (Utilities|FlowControl|DoOnce false
      (:Completed
        (Character|LaunchCharacter "0.000000,0.000000,1200.000000" false true)))))

(event Input|EnhancedActionEvents|EnhancedInputActionFreeze
  (params (ActionValue :type Boolean) (ElapsedSeconds :type Float%20%28double-precision%29) (TriggeredSeconds :type Float%20%28double-precision%29) (InputAction :type Input%20Action%20Object%20Reference :default "/Game/OverwatchCharacters/Okito/Inputs/Freeze.Freeze"))
  (bind _firstpersoncamera (Variables|Default|GetFirstPersonCamera))
  (bind _returnvalue (Transformation|GetWorldRotation _firstpersoncamera))
  (:Triggered
    (Audio|SpawnSound2D "/Game/Sound/magic-spell-6005.magic-spell-6005" 1.0 1.0 0.0 0)
    (bind _returnvalue_2 (Game|SpawnActorfromClass "/Game/FirstPerson/Blueprints/BP_SnowBall.BP_SnowBall_C" (Math|Transform|MakeTransform (Transformation|GetWorldLocation (Variables|Default|GetSpawnPoint)) _returnvalue "1.000000,1.000000,1.000000") "Undefined" "OverrideRootScale" 0 0))
    (Physics|SetPhysicsLinearVelocity (Variables|/Game/FirstPerson/Blueprints/BP_SnowBall.BP_SnowBall_C|GetSphere _returnvalue_2) (* (Math|Vector|GetForwardVector _returnvalue) 5e+03) false "None")))

(event Input|EnhancedActionEvents|EnhancedInputActionFire
  (params (ActionValue :type Boolean) (ElapsedSeconds :type Float%20%28double-precision%29) (TriggeredSeconds :type Float%20%28double-precision%29) (InputAction :type Input%20Action%20Object%20Reference :default "/Game/OverwatchCharacters/Okito/Inputs/Fire.Fire"))
  (bind _firstpersoncamera (Variables|Default|GetFirstPersonCamera))
  (bind _returnvalue (Transformation|GetWorldRotation _firstpersoncamera))
  (:Triggered
    (Audio|SpawnSound2D "/Game/Sound/fireball-whoosh.fireball-whoosh" 1.0 1.0 0.0 0)
    (bind _returnvalue_2 (Game|SpawnActorfromClass "/Game/FirstPerson/Blueprints/BP_FireBall.BP_FireBall_C" (Math|Transform|MakeTransform (Transformation|GetWorldLocation (Variables|Default|GetSpawnPoint)) _returnvalue "1.000000,1.000000,1.000000") "Undefined" "OverrideRootScale" 0 0))
    (Physics|SetPhysicsLinearVelocity (Variables|/Game/FirstPerson/Blueprints/BP_FireBall.BP_FireBall_C|GetSphere _returnvalue_2) (* (Math|Vector|GetForwardVector _returnvalue) 5e+03) false "None")))

(event EventBeginPlay
  (|CallParentFunction)
  ;[0 0 0] arme spécifique de genji
  (AddComponent|AddBPWeaponComponent false))

(event EventInitializeMe
  ;[0 0 0] on ajoute le contexte okito
  (bind _asplayer_controller (Utilities|Casting|CastToPlayerController (Pawn|GetController)))
  (Utilities|IsValid (PlayerController|LocalPlayerSubsystems|GetEnhancedInputLocalPlayerSubsystem _asplayer_controller)
    (:Is%20Valid
      (Input|AddMappingContext (PlayerController|LocalPlayerSubsystems|GetEnhancedInputLocalPlayerSubsystem _asplayer_controller) "/Game/OverwatchCharacters/Okito/IMC_Okito.IMC_Okito" 1 "(bIgnoreAllPressedKeysUntilRelease=True,bForceImmediately=False)")
      (bind _returnvalue (UserInterface|CreateWidget "/Game/OverwatchCharacters/Okito/Tuto_Okito.Tuto_Okito_C"))
      (UserInterface|Viewport|AddtoViewport _returnvalue 0)
      (Utilities|FlowControl|Delay 5.0)
      (Widget|RemovefromParent _returnvalue))))

(fn ConstructionScript
  (|CallParentFunction))